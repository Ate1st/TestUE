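; BaseItem is an item Actor, apparently a parent class, that can be hidden from the world and restored at a given location.
; Hide stops mesh physics, reattaches it to the root, teleports both far out of bounds and hides them instead of destroying the actor.
; Unhide teleports them back, shows them and re-enables physics, returning whether that succeeded.
; GetMesh finds the mesh component by class, and Hidden is never cleared on Unhide.
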(fn `GetMesh`
  (returns (Mesh :type "MeshComponent Object Reference"))
  (return (`self.GetComponentByClass` self "/Script/Engine.MeshComponent")))

(fn `Hide`
  (returns (Hidden :type Boolean))
  (bind _mesh (`self.GetMesh`))
  (bind _defaultsceneroot (`self.DefaultSceneRoot`))
  (if (not (`self.SetPhysics` false))
    (`self.K2_SetActorLocation` (999999.0 999999.0 999999.0) false true)
    (`SceneComponent.K2_SetWorldLocation` _mesh (`self.K2_GetActorLocation` self) false true)
    (`SceneComponent.K2_SetWorldRotation` _mesh (`self.K2_GetActorRotation` self) false false)
    (`SceneComponent.SetHiddenInGame` _defaultsceneroot true true)
    (set `self.Hidden` true)
    (return (`SceneComponent.bHiddenInGame` _defaultsceneroot))
    (else
      (return false))))

(fn `SetPhysics`
  (params (Enable :type Boolean))
  (returns (Enabled :type Boolean))
  (bind _mesh (`self.GetMesh`))
  (if Enable
    (`PrimitiveComponent.SetSimulatePhysics` _mesh true)
    (else
      (`PrimitiveComponent.SetSimulatePhysics` _mesh false)
      (`SceneComponent.K2_AttachToComponent` _mesh (`self.DefaultSceneRoot`) "None" "KeepRelative" "KeepRelative" "KeepRelative" true)))
  (return (`SceneComponent.IsSimulatingPhysics` _mesh "None")))

(fn `Unhide`
  (params (Location :type "Vector Structure"))
  (returns (Hidden :type Boolean))
  (locals (L_Location :type "Vector Structure") (L_LocationChanged :type Boolean))
  (bind _output_get (set `local.L_Location` Location))
  (bind (_sweephitresult _returnvalue) (`self.K2_SetActorLocation` self _output_get false true))
  (set `local.L_LocationChanged` _returnvalue)
  (`SceneComponent.K2_SetWorldLocation` (`self.GetMesh`) (`local.L_Location`) false true)
  (`SceneComponent.SetHiddenInGame` (`self.DefaultSceneRoot`) false true)
  (if (and (`self.SetPhysics` true) (`local.L_LocationChanged`))
    (return true)
    (else
      (return false))))

(fn `UserConstructionScript`)